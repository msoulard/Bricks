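; BPC_PawnFire is a component that gives its owning pawn a projectile fire action.
; FFire spawns a BP_Projectile at the pawn's Arrow location with the pawn's rotation, passing it the pawn's forward vector.
; A forward Visibility line trace with persistent debug drawing remains in the function but is disconnected, and the event graph holds only disabled default events.
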(fn `F_Fire`
  (locals (distance :type Integer :default 1000))
  (bind _pawnowner (`self.PawnOwner`))
  (`|SpawnActorFromClass` "/Game/01_Scripts/BP_Projectile.BP_Projectile_C" (`KismetMathLibrary.MakeTransform` (`SceneComponent.K2_GetComponentLocation` (`/Game/01_Scripts/BP_Pawn.Arrow` _pawnowner)) (`Actor.K2_GetActorRotation` _pawnowner)) "Undefined" "MultiplyWithRoot" null (`Actor.GetActorForwardVector` _pawnowner) null))