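; BPC_PawnMovement is a pawn component that slides its owner sideways along its right vector at a set speed.
; SetMovement box-traces at the owner's left or right bound component, chosen by input, and moves the pawn without sweep only when nothing is hit.
; It also caches the start location on BeginPlay and exposes helpers to zero or flip TargetForwardValue, which the movement here does not read.
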(event `self.ReceiveBeginPlay`
  (`parent.ReceiveBeginPlay`)
  (set `self.DefaultLocation` (`Actor.K2_GetActorLocation` (`self.PawnOwner`))))

(fn `F_ChangeTargetForwardValue`
  (set `self.TargetForwardValue` (* (`self.TargetForwardValue`) -1.0)))

(fn `F_ResetTargetForwardValue`
  (set `self.TargetForwardValue` 0.0))

(fn `F_SetMovement`
  (params (RightValue :type "Float (double-precision)"))
  (bind _pawnowner (`self.PawnOwner`))
  (bind _pawnowner_2 (`self.PawnOwner`))
  (bind _returnvalue (`SceneComponent.K2_GetComponentLocation` (select `bool` (== RightValue 1.0) :`false` (`/Game/01_Scripts/BP_Pawn.CTRL_LeftBound` _pawnowner) :`true` (`/Game/01_Scripts/BP_Pawn.CTRL_RightBound` _pawnowner))))
  (bind (_outhit _returnvalue_2) (`KismetSystemLibrary.BoxTraceSingle` _returnvalue _returnvalue (1.0 1.0 1.0) (struct) "TraceTypeQuery1"))
  (if (not _returnvalue_2)
    (`Actor.K2_SetActorLocation` _pawnowner_2 (+ (`Actor.K2_GetActorLocation` _pawnowner_2) (* (`Actor.GetActorRightVector` _pawnowner_2) RightValue (`self.Speed`))) false false)))