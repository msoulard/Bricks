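; BP_Asteroid is a short-lived asteroid actor that drifts across the XY plane in a random direction.
; Tick moves it by a fixed per-frame step without delta time or sweep, and wall collisions negate its speed to bounce it straight back.
; It destroys itself on a timer or the game instance's Replay dispatcher, while a hit first broadcasts its Destroyed dispatcher.
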(event `self.ReceiveBeginPlay`
  (bind (_returnvalue_x _returnvalue_y) (`KismetMathLibrary.BreakVector` (`KismetMathLibrary.RandomUnitVector`)))
  (set `self.ForwardVector` (`KismetMathLibrary.MakeVector` _returnvalue_x _returnvalue_y))
  (`KismetSystemLibrary.K2_SetTimerDelegate` (delegate `E_Death`) 4.0)
  (add `/Game/01_Scripts/BP_GameInstance.ED_Replay` (`/Game/01_Scripts/BP_Utils.F_GetGameinstance`) (delegate `E_Replay`)))

(event `E_Death`
  (`self.K2_DestroyActor`))

(event `E_Replay`
  (`self.K2_DestroyActor`))

(event `self.ReceiveTick`
  (params (DeltaSeconds :type "Float (single-precision)"))
  (`self.K2_SetActorLocation` (+ (`self.K2_GetActorLocation`) (* (`self.ForwardVector`) (`self.Speed`)))))

(event `E_Hit`
  (`self.ED_Destroyed` self)
  (`self.K2_DestroyActor`))

(event `E_CollisionWall`
  (bind _output_get (set `self.Speed` (* (`self.Speed`) -1.0)))
  (`self.K2_SetActorLocation` (+ (`self.K2_GetActorLocation`) (* (`self.ForwardVector`) _output_get))))

(fn `UserConstructionScript`)