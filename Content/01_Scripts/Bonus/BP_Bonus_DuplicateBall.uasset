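; BP_Bonus_DuplicateBall is a bonus powerup that adds another ball to play.
; When executed, it has the pawn spawn a bonus-flagged projectile at the location of the first projectile in the pawn's list.
; The spawn and the parent's powerup logic run only while the projectile count is within a small cap.
; BeginPlay calls EDDestroy and EDWin.
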(event `self.ReceiveBeginPlay`
  (`self.ED_Destroy`)
  (`self.ED_Win`))

(event `self.E_ExecutePowerup`
  (bind _pawn (`/Game/01_Scripts/BP_Utils.F_GetPawn`))
  (bind _allprojectiles (`/Game/01_Scripts/BP_Pawn.AllProjectiles` _pawn))
  (if (<= (`KismetArrayLibrary.Array_Length` _allprojectiles) 8)
    (`/Game/01_Scripts/BP_Pawn.E_SpawnProjectile` _pawn (`self.K2_GetActorLocation` (`|GetArrayItem` _allprojectiles)) true)
    (`parent.E_ExecutePowerup`)))

(fn `UserConstructionScript`
  (`parent.UserConstructionScript`))