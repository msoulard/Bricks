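; A bonus pickup that grows or shrinks the pawn's size when collected.
; On BeginPlay it randomly picks grow or shrink, colors its sphere green or red to show which, and calls the inherited destroy event.
; Executing the powerup steps the pawn's Size up or down within a clamped range, then runs the parent powerup logic.
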(event `self.ReceiveBeginPlay`
  (bind _output_get (set `self.Bigger` (`KismetMathLibrary.RandomBool`)))
  (`MeshComponent.SetVectorParameterValueOnMaterials` (`self.Sphere`) "Color" (`KismetMathLibrary.SelectVector` (0.0 1.0 0.0) (1.0 0.0 0.0) _output_get))
  (`self.ED_Destroy`))

(event `self.E_ExecutePowerup`
  (bind _pawn (`/Game/01_Scripts/BP_Utils.F_GetPawn`))
  (set `/Game/01_Scripts/BP_Pawn.Size` (`KismetMathLibrary.Clamp` (+ (`/Game/01_Scripts/BP_Pawn.Size` _pawn) (`KismetMathLibrary.SelectInt` 1 -1 (`self.Bigger`))) -3 5) _pawn)
  (`parent.E_ExecutePowerup`))

(fn `UserConstructionScript`
  (`parent.UserConstructionScript`))