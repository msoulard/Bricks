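; BP_Bonus is a moving powerup pickup actor that removes itself when executed or out of play.
; Each tick it shifts along its Arrow's forward vector by Speed, without sweep or delta-time scaling.
; It destroys itself on overlapping a DeadZone-tagged actor or when E_ExecutePowerup fires, which applies no effect here.
; ED_Destroy binds E_Destroy to the pawn's EDDied event, so the pawn's death also destroys the bonus.
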(event `ED_Destroy`
  (add `/Game/01_Scripts/BP_Pawn.ED_Died` (`/Game/01_Scripts/BP_Utils.F_GetPawn`) (delegate `E_Destroy`)))

(event `E_Destroy`
  (`self.K2_DestroyActor`))

(event `self.ReceiveTick`
  (params (DeltaSeconds :type "Float (single-precision)"))
  (`self.K2_SetActorLocation` (+ (`self.K2_GetActorLocation`) (* (`SceneComponent.GetForwardVector` (`self.Arrow`)) (`self.Speed`)))))

(event `self.ReceiveActorBeginOverlap`
  (params (OtherActor :type "Actor Object Reference"))
  (if (`self.ActorHasTag` OtherActor "DeadZone")
    (`self.K2_DestroyActor`)))

(event `E_ExecutePowerup`
  (`self.K2_DestroyActor`))

(fn `UserConstructionScript`)