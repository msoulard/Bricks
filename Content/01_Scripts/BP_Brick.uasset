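; BP_Brick is a breakable brick, apparently for a Breakout-style game, that randomly decides on BeginPlay and reset whether it holds a bonus.
; E_Hit hides it, disables collision, updates BricksManager and ScoreManager through the game instance, and plays destroy effects.
; A bonus brick then spawns a randomly chosen bigger-bar or smaller-bar pickup.
; The brick is never destroyed, so E_Reset restores it for reuse.
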(event `self.ReceiveBeginPlay`
  (set `self.HasBonus` (>= (`KismetMathLibrary.RandomFloat`) 0.8)))

(event `E_Hit`
  (bind _bonusclass (`self.F_GetRandomBonus`))
  (bind _returnvalue (`self.K2_GetActorLocation`))
  (bind _returnvalue_2 (`self.K2_GetActorLocation`))
  (bind _bricksmanager (`/Game/01_Scripts/BP_GameInstance.BricksManager` (`/Game/01_Scripts/BP_Utils.F_GetGameInstance`)))
  (`self.SetActorEnableCollision` false)
  (`SceneComponent.SetVisibility` (`self.DefaultSceneRoot`) false true)
  (set `self.Active` false)
  (set `/Game/01_Scripts/BP_BricksManager.BricksDeactivate` (+ (`/Game/01_Scripts/BP_BricksManager.BricksDeactivate` _bricksmanager) 1) _bricksmanager)
  (`/Game/01_Scripts/BP_ScoreManager.E_SetScore` (`/Game/01_Scripts/BP_GameInstance.ScoreManager` (`/Game/01_Scripts/BP_Utils.F_GetGameInstance`)))
  (`NiagaraFunctionLibrary.SpawnSystemAtLocation` "/Game/05_Particules/NS_DestroyBrick.NS_DestroyBrick" _returnvalue_2)
  (`GameplayStatics.PlaySoundAtLocation` "/Game/06_Sounds/SC_DestroyBrick.SC_DestroyBrick" _returnvalue_2 (struct) 1.0 1.0 0.0 null null null null)
  (if (`self.HasBonus`)
    (bind _asbp_bonus_bigger_bar (castclass `/Game/01_Scripts/BP_Bonus_BiggerBar` _bonusclass)
      (:`then`
        (`|SpawnActorFromClass` _asbp_bonus_bigger_bar (`KismetMathLibrary.Conv_VectorToTransform` _returnvalue) "Undefined" "MultiplyWithRoot" null null))
      (:`CastFailed`
        (bind _asbp_bonus_smaller_bar (castclass `/Game/01_Scripts/BP_Bonus_SmallerBar` _bonusclass))
        (`|SpawnActorFromClass` _asbp_bonus_smaller_bar (`KismetMathLibrary.Conv_VectorToTransform` _returnvalue) "Undefined" "MultiplyWithRoot" null null)))))

(event `E_Reset`
  (`self.SetActorEnableCollision` true)
  (`SceneComponent.SetVisibility` (`self.DefaultSceneRoot`) true true)
  (set `self.Active` true)
  (set `self.HasBonus` (>= (`KismetMathLibrary.RandomFloat`) 0.8)))

(fn `F_GetRandomBonus`
  (returns (BonusClass :type "Object Class Reference"))
  (return (`/Game/01_Scripts/BP_MacroLibraray.M_GetRandomInArray` (`|MakeArray` "/Game/01_Scripts/BP_Bonus_BiggerBar.BP_Bonus_BiggerBar_C" "/Game/01_Scripts/BP_Bonus_SmallerBar.BP_Bonus_SmallerBar_C" :!type "Object Class Reference"))))

(fn `UserConstructionScript`)