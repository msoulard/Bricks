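; Manager actor that spawns asteroids and splits them when destroyed, registering itself with the game instance on begin play.
; A looping one-second timer spawns a random-sized BP_Asteroid, picking position and rotation from random spawn points.
; Each spawn's destroyed event is bound back to the manager, which rebroadcasts the type and replaces non-small asteroids with two of the next size down.
; A shared spawn function maps type to scale; the bound replay handler is empty.
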(event `self.ReceiveBeginPlay`
  (set `/Game/01_Scripts/BP_GameInstance.AsteroidManager` self (`/Game/01_Scripts/BP_Utils.F_GetGameinstance`))
  (`KismetSystemLibrary.K2_SetTimerDelegate` (delegate `E_SpawnAsteroidLoop`) 1.0 true)
  (add `/Game/01_Scripts/BP_GameInstance.ED_Replay` (`/Game/01_Scripts/BP_Utils.F_GetGameinstance`) (delegate `E_Replay`)))

(event `E_Replay`)

(event `E_SpawnAsteroidLoop`
  (bind _element (`/Game/01_Scripts/BP_MacroLibraray.M_GetRandomInArray` (`self.SpawnPoints`)))
  (bind _asteroid (`self.F_SpawnAsteroid` (`self.K2_GetActorLocation` _element) (`self.K2_GetActorRotation` _element) (`/Game/01_Scripts/BP_MacroLibraray.M_GetRandomInArray` (`|MakeArray` "NewEnumerator0" "NewEnumerator1" "NewEnumerator2" :!type "/Game/01_Scripts/Enums/E_AsteroidType Enum"))))
  (`/Engine/EditorBlueprintResources/StandardMacros.IsValid` _asteroid
    (:`Is Valid`
      (add `/Game/01_Scripts/BP_Asteroid.ED_Destroyed` _asteroid (delegate `E_ActionOnAsteroidDestroyed`)))))

(event `E_ActionOnAsteroidDestroyed`
  (params (Asteroid :type "/Game/01_Scripts/BP_Asteroid Object Reference"))
  (bind _returnvalue (`self.K2_GetActorLocation` Asteroid))
  (bind _returnvalue_2 (`self.K2_GetActorRotation` Asteroid))
  (bind _type (`/Game/01_Scripts/BP_Asteroid.Type` Asteroid))
  (bind _returnvalue_3 (select `/Game/01_Scripts/Enums/E_AsteroidType` _type :`NewEnumerator0` "NewEnumerator1" :`NewEnumerator1` "NewEnumerator2" :`NewEnumerator2` "NewEnumerator0" :!type "/Game/01_Scripts/Enums/E_AsteroidType Enum"))
  (`self.ED_AsteroidDestroyed` _type)
  (if (`|EnumInequality` _type "NewEnumerator2")
    (`|ExecutionSequence`
      (:`then_0`
        (bind _asteroid (`self.F_SpawnAsteroid` _returnvalue _returnvalue_2 _returnvalue_3))
        (`/Engine/EditorBlueprintResources/StandardMacros.IsValid` _asteroid
          (:`Is Valid`
            (add `/Game/01_Scripts/BP_Asteroid.ED_Destroyed` _asteroid (delegate `E_ActionOnAsteroidDestroyed`)))))
      (:`then_1`
        (bind _asteroid_2 (`self.F_SpawnAsteroid` _returnvalue _returnvalue_2 _returnvalue_3))
        (`/Engine/EditorBlueprintResources/StandardMacros.IsValid` _asteroid_2
          (:`Is Valid`
            (add `/Game/01_Scripts/BP_Asteroid.ED_Destroyed` _asteroid_2 (delegate `E_ActionOnAsteroidDestroyed`))))))))

(fn `F_SpawnAsteroid`
  (params (Position :type "Vector Structure") (Rotation :type "Rotator Structure") (Type :type "/Game/01_Scripts/Enums/E_AsteroidType Enum" :default "NewEnumerator0"))
  (returns (Asteroid :type "/Game/01_Scripts/BP_Asteroid Object Reference"))
  (locals (Scale :type "Vector Structure"))
  (switch `/Game/01_Scripts/Enums/E_AsteroidType` Type
    (:`NewEnumerator0`
      (set `local.Scale` (1.0 1.0 0.2)))
    (:`NewEnumerator1`
      (set `local.Scale` (0.5 0.5 0.1)))
    (:`NewEnumerator2`
      (set `local.Scale` (0.25 0.25 0.05))))
  (bind _returnvalue (`|SpawnActorFromClass` "/Game/01_Scripts/BP_Asteroid.BP_Asteroid_C" (`KismetMathLibrary.MakeTransform` Position Rotation (`local.Scale`)) "AlwaysSpawn" "MultiplyWithRoot" null Type null))
  (return _returnvalue))

(fn `UserConstructionScript`)