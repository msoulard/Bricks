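; Player paddle pawn for a brick-breaker game, owning lives, balls and paddle width.
; BeginPlay polls until the UI exists, then binds replay and win events and spawns an attached ball.
; Launch detaches it along a random arrow direction; bonus balls launch immediately, and losing the last ball costs a life or triggers game over.
; Movement goes through BPCMovement, overlaps execute bonuses, and Tick interpolates width toward the Size-driven target.
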(event OnComponentBeginOverlap(Cube)
  (params (OverlappedComponent :type Primitive%20Component%20Object%20Reference) (OtherActor :type Actor%20Object%20Reference) (OtherComp :type Primitive%20Component%20Object%20Reference) (OtherBodyIndex :type Integer) (bFromSweep :type Boolean) (SweepResult :type Hit%20Result%20Structure%20%28by%20ref%29))
  (bind _asbp_bonus (Utilities|Casting|CastToBP_Bonus OtherActor))
  (Default|EExecutePowerup _asbp_bonus))

(event Custom|E_LaunchProjectile
  (bind _projectile (Variables|Default|GetProjectile))
  (Utilities|IsValid _projectile :!label _label
    (:Is%20Valid
      (Default|ELaunch _projectile (Utilities|MGetRandominArray (Utilities|Array|MakeArray (Math|Vector|GetForwardVector (Variables|Default|GetArrowLeft)) (Math|Vector|GetForwardVector (Variables|Default|GetArrowLeft1)) (Math|Vector|GetForwardVector (Variables|Default|GetArrowLeft2)) (Math|Vector|GetForwardVector (Variables|Default|GetArrowRight)) (Math|Vector|GetForwardVector (Variables|Default|GetArrowRight1)) (Math|Vector|GetForwardVector (Variables|Default|GetArrowRight2)))))
      (Transformation|DetachFromActor _projectile "KeepWorld" "KeepWorld" "KeepWorld"))
    (:Is%20Not%20Valid
      (Utilities|FlowControl|Delay 0.2)
      (goto _label))))

(event Custom|E_Win
  (Utilities|Array|Clear (Variables|Default|GetAllProjectiles)))

(event Custom|E_ResetPawn
  (CallFunction|FResetPawn)
  (CallFunction|ESpawnProjectile (Transformation|GetWorldLocation (Variables|Default|GetBillboard)) false))

(event Custom|E_Move
  (params (RightValue :type Float%20%28double-precision%29))
  (Default|FSetMovement (Variables|Default|GetBPC_Movement) RightValue))

(event Custom|E_SpawnProjectile
  (params (Location :type Vector) (FromBonus :type Boolean))
  (bind _returnvalue (Game|SpawnActorfromClass "/Game/01_Scripts/BP_Projectile.BP_Projectile_C" (Math|Transform|MakeTransform Location) "Undefined" "MultiplyWithRoot" 0 "0.000000,0.000000,0.000000" 0))
  (bind _output_get (Variables|Default|SetProjectile _returnvalue))
  (Transformation|AttachActorToActor _output_get self "None" "KeepWorld" "KeepWorld" "KeepWorld" true)
  (if FromBonus
    (CallFunction|ELaunchProjectile))
  (Utilities|Array|Add (Variables|Default|GetAllProjectiles) (Variables|Default|GetProjectile))
  (EventDispatchers|BindEventtoEDDead (Variables|Default|GetProjectile) (delegate Custom|E_Destroy)))

(event Custom|E_Destroy
  (params (Projectile :type BP%20Projectile%20Object%20Reference))
  (bind _vie (Variables|Default|GetVie))
  (bind _allprojectiles (Variables|Default|GetAllProjectiles))
  (Utilities|Array|RemoveItem _allprojectiles Projectile)
  (Actor|DestroyActor Projectile)
  (if (== (Utilities|Array|Length _allprojectiles) 0)
    (Audio|PlaySound2D "/Game/06_Sounds/SC_TouchWallDied.SC_TouchWallDied" 1.0 1.0 0.0 0 0)
    (bind _result (Math|Integer|DecrementInt _vie)
      (:%20%20
        (Default|FSetVie (Variables|Default|GetUIMain) _result)
        (Default|CallEDDied)
        (CallFunction|FResetScale)
        (if (== (Math|Integer|Clamp(Integer) _vie 0 5) 0)
          (Default|EGameOver (CallFunction|FGetGameInstance))
          (else
            (CallFunction|ESpawnProjectile (Transformation|GetWorldLocation (Variables|Default|GetBillboard)) false)))))))

(event Custom|E_HandleSize
  (bind _cube (Variables|Default|GetCube))
  (bind _returnvalue (Transformation|GetWorldScale _cube))
  ;[1 1 1] Handle size
  (Transformation|SetRelativeScale3D _cube (Math|Vector|MakeVector (.x _returnvalue) (Math|Interpolation|FInterptoConstant (.y _returnvalue) (+ (Variables|Default|GetDefaultSize) (* (Variables|Default|GetSize) (Variables|Default|GetSizeFactor))) (Utilities|Time|GetWorldDeltaSeconds) (Variables|Default|GetSizeSpeed)) (.z _returnvalue))))

(event EventBeginPlay
  (Utilities|IsValid (Variables|/Game/01_Scripts/BP_GameInstance.BP_GameInstance_C|GetUIMain (CallFunction|FGetGameInstance)) :!label _label
    (:Is%20Valid
      (Variables|Default|SetVie 5)
      (Variables|Default|SetUIMain (Variables|/Game/01_Scripts/BP_GameInstance.BP_GameInstance_C|GetUIMain (CallFunction|FGetGameInstance)))
      (Default|FSetVie (Variables|/Game/01_Scripts/BP_GameInstance.BP_GameInstance_C|GetUIMain (CallFunction|FGetGameInstance)) (Variables|Default|GetVie))
      (Variables|Default|SetDefaultLocation (Transformation|GetActorLocation))
      (EventDispatchers|BindEventtoEDReplay (CallFunction|FGetGameInstance) (delegate Custom|E_ResetPawn))
      (Variables|Default|SetDefaultSize (.y (Variables|/Script/Engine.SceneComponent|GetRelativeScale3D (Variables|Default|GetCube))))
      (CallFunction|ESpawnProjectile (Transformation|GetWorldLocation (Variables|Default|GetBillboard)) false)
      (EventDispatchers|BindEventtoEDWin (Variables|/Game/01_Scripts/BP_GameInstance.BP_GameInstance_C|GetBricksManager (CallFunction|FGetGameInstance)) (delegate Custom|E_Win)))
    (:Is%20Not%20Valid
      (Utilities|FlowControl|Delay 0.2)
      (goto _label))))

(event EventTick
  (params (DeltaSeconds :type Float%20%28single-precision%29))
  (CallFunction|EHandleSize))

(event Input|KeyboardEvents|DebugKeyA
  (params (Key :type Key%20Structure :default "None") (ActionValue :type Input%20Action%20Value%20Structure))
  (:Pressed
    (bind _outactors (Actor|GetAllActorsOfClass "/Game/01_Scripts/BP_BricksManager.BP_BricksManager_C"))
    (Default|EDebugWin (Utilities|Array|Get(acopy) _outactors))))

(fn ConstructionScript)

(fn FResetPawn
  (Transformation|SetActorLocation (Variables|Default|GetDefaultLocation) false false)
  (Variables|Default|SetVie 5)
  (Default|FSetVie (Variables|Default|GetUIMain) (Variables|Default|GetVie))
  (CallFunction|FResetScale)
  (Utilities|Array|Clear (Variables|Default|GetAllProjectiles)))

(fn FResetScale
  (bind _cube (Variables|Default|GetCube))
  (bind _returnvalue (Transformation|GetWorldScale _cube))
  (Transformation|SetRelativeScale3D _cube (Math|Vector|MakeVector (.x _returnvalue) (Variables|Default|GetDefaultSize) (.z _returnvalue)))
  (Variables|Default|SetSize 0))