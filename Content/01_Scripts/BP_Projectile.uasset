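; Brick-breaker ball that bounces around the level, hitting bricks and reporting contact with dead zones.
; Tick moves it manually without physics, sphere-tracing the next position and mirroring its 2D direction on the impact normal.
; Hits notify BP_Brick or fire the dead dispatcher for DeadZone-tagged actors.
; E_Launch starts it only when stopped; replay restores its start location, winning stops it, and helper functions place it at the pawn.
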(event `self.ReceiveBeginPlay`
  (bind _gameinstance (`/Game/01_Scripts/BP_Utils.F_GetGameInstance`))
  (set `self.DefaultLocation` (`self.K2_GetActorLocation`))
  (add `/Game/01_Scripts/BP_GameInstance.ED_Replay` _gameinstance (delegate `E_Replay`))
  (add `/Game/01_Scripts/BP_BricksManager.ED_Win` (`/Game/01_Scripts/BP_GameInstance.BricksManager` _gameinstance) (delegate `E_Win`)))

(event `E_Replay`
  (`self.F_Reset`))

(event `E_Win`
  (set `self.Speed` 0.0)
  (`GameplayStatics.PlaySound2D` "/Game/06_Sounds/SC_Win.SC_Win" 1.0 1.0 0.0 null null))

(event `self.ReceiveTick`
  (params (DeltaSeconds :type "Float (single-precision)"))
  (bind (_forwardvector_x _forwardvector_y) (`KismetMathLibrary.BreakVector` (`self.ForwardVector`)))
  (bind _returnvalue (+ (`self.K2_GetActorLocation`) (* (`self.ForwardVector`) (`self.Speed`))))
  (bind (_outhit _returnvalue_2) (`KismetSystemLibrary.SphereTraceSingle` :`Start` _returnvalue :`End` _returnvalue :`Radius` 10.0 :`TraceChannel` "TraceTypeQuery1" :`bIgnoreSelf` false))
  (if _returnvalue_2
    (`|ExecutionSequence`
      (:`then_0`
        (bind (_bblockinghit _binitialoverlap _time _distance _location _impactpoint _normal _impactnormal _physmat _hitactor) (`GameplayStatics.BreakHitResult` _outhit))
        (if (`self.ActorHasTag` _hitactor "DeadZone")
          (`self.ED_Dead` self)))
      (:`then_1`
        (bind (_returnvalue_x _returnvalue_y) (`KismetMathLibrary.BreakVector` (`KismetMathLibrary.MirrorVectorByNormal` (`KismetMathLibrary.MakeVector` _forwardvector_x _forwardvector_y) (`KismetMathLibrary.MakeVector` (.x _impactnormal) (.y _impactnormal)))))
        (bind (_returnvalue_x_2 _returnvalue_y_2 _returnvalue_z) (`KismetMathLibrary.BreakVector` (`KismetMathLibrary.Normal` (`KismetMathLibrary.MakeVector` _returnvalue_x _returnvalue_y))))
        (set `self.ForwardVector` (`KismetMathLibrary.MakeVector` _returnvalue_x_2 _returnvalue_y_2 _returnvalue_z))
        (`self.K2_SetActorLocation` (+ (`self.K2_GetActorLocation`) (* (`self.ForwardVector`) (`self.Speed`)))))
      (:`then_2`
        (bind _asbp_brick (cast `/Game/01_Scripts/BP_Brick` _hitactor))
        (`/Game/01_Scripts/BP_Brick.E_Hit` _asbp_brick)))
    (else
      (`self.K2_SetActorLocation` _returnvalue))))

(event `E_Launch`
  (params (ForwarVector :type "Vector Structure"))
  (if (== (`self.Speed`) 0.0)
    (`self.F_Launch` ForwarVector)))

(fn `F_Launch`
  (params (ForwardVector :type "Vector Structure"))
  (set `self.ForwardVector` (`KismetMathLibrary.Normal` ForwardVector))
  (set `self.Speed` 17.5))

(fn `F_OnPawn`
  (bind (_returnvalue_x _returnvalue_y _returnvalue_z) (`KismetMathLibrary.BreakVector` (`self.K2_GetActorLocation` (`/Game/01_Scripts/BP_Utils.F_GetPawn`))))
  (`self.K2_SetActorLocation` (`KismetMathLibrary.MakeVector` (+ _returnvalue_x 40.0) _returnvalue_y _returnvalue_z)))

(fn `F_Reset`
  (`self.K2_SetActorLocation` (`self.DefaultLocation`)))

(fn `F_ResetProjectile`
  (bind (_returnvalue_x _returnvalue_y _returnvalue_z) (`KismetMathLibrary.BreakVector` (`self.K2_GetActorLocation` (`GameplayStatics.GetPlayerPawn` 0))))
  (set `self.Speed` 0.0)
  (set `self.ForwardVector` (0.0 0.0 0.0))
  (`self.K2_SetActorLocation` (`KismetMathLibrary.MakeVector` (+ _returnvalue_x 40.0) _returnvalue_y _returnvalue_z)))

(fn `UserConstructionScript`)