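; BP_SaveGame is a save game Blueprint that turns a Score map of names and values into display text for a score list.
; FGetScores loops over the map's keys, looks up each score and appends a colon-separated name and score pair to TextScoresNames.
; It returns the accumulated text, with entries in key order and no sorting by score.
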(fn `F_GetScores`
  (returns (Output_Get :type Text))
  (locals (TextScoresNames :type Text))
  (bind _score (`self.Score`))
  (bind _keys (`BlueprintMapLibrary.Map_Keys` _score))
  (for _array_element _keys
    (set `local.TextScoresNames` (`KismetTextLibrary.Conv_StringToText` (`KismetStringLibrary.Concat_StrStr` (`KismetTextLibrary.Conv_TextToString` (`local.TextScoresNames`)) (`KismetStringLibrary.Concat_StrStr` _array_element " : " (`KismetStringLibrary.Conv_IntToString` (`BlueprintMapLibrary.Map_Find` _score _array_element)) " \n")))))
  (return (`local.TextScoresNames`)))