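; BP_BricksManager tracks the level's breakable bricks and triggers a win when all are destroyed.
; On BeginPlay it registers with the game instance, then resets every default brick and rebuilds the current list from breakable ones, repeating this on the replay dispatcher.
; Each brick's destroyed dispatcher removes it from that list; an empty list calls the game instance's win and fires its own win dispatcher.
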(event `self.ReceiveBeginPlay`
  (bind _gameinstance (`/Game/01_Scripts/BP_Utils.F_GetGameInstance`))
  (set `/Game/01_Scripts/BP_GameInstance.BricksManager` self _gameinstance)
  (`self.F_Init`)
  (add `/Game/01_Scripts/BP_GameInstance.ED_Replay` _gameinstance (delegate `E_Replay`))
  (for _array_element (`self.DefaultBricks`)
    (add `/Game/01_Scripts/BP_Brick.ED_Destroyed` _array_element (delegate `E_ActionOnBrickDestroyed`))))

(event `E_DebugWin`
  (`/Game/01_Scripts/BP_GameInstance.E_Win` (`/Game/01_Scripts/BP_Utils.F_GetGameInstance`) :!label _label)
  (`self.ED_Win`))

(event `E_ActionOnBrickDestroyed`
  (params (DestroyedBrick :type "/Game/01_Scripts/BP_Brick Object Reference"))
  (bind _currentbricks (`self.CurrentBricks`))
  (bind _returnvalue (`KismetArrayLibrary.Array_Length` _currentbricks))
  (`KismetArrayLibrary.Array_RemoveItem` _currentbricks DestroyedBrick)
  (`KismetSystemLibrary.PrintString` (`KismetStringLibrary.Conv_IntToString` _returnvalue))
  (if (<= _returnvalue 0)
    (goto _label)))

(event `E_Replay`
  (`self.F_Init`))

(fn `F_Init`
  (bind _defaultbricks (`self.DefaultBricks`))
  (`KismetArrayLibrary.Array_Clear` (`self.CurrentBricks`))
  (for _array_element _defaultbricks
    (`/Game/01_Scripts/BP_Brick.E_Reset` _array_element))
  (for _array_element_2 _defaultbricks
    (if (`/Game/01_Scripts/BP_Brick.IsBreakable` _array_element_2)
      (`KismetArrayLibrary.Array_Add` (`self.CurrentBricks`) _array_element_2)))
  (`KismetSystemLibrary.PrintString` (`KismetStringLibrary.Conv_IntToString` (`KismetArrayLibrary.Array_Length` (`self.CurrentBricks`))) true true (struct :`R` 1.0 :`B` 0.069327 :`A` 1.0) 5.0))

(fn `UserConstructionScript`)