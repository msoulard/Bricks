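; Player controller that routes Enhanced Input actions to the controlled pawn.
; On BeginPlay it caches the pawn and, if the input subsystem is valid, adds the player mapping context and triggers the game instance's main initialization.
; Movement input passes its value to the pawn's move event, and spawn input calls the pawn's spawn event, leaving the behavior itself to the pawn.
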(event `self.ReceiveBeginPlay`
  (bind _returnvalue (subsystem `EnhancedInputLocalPlayerSubsystem`))
  (set `self.ControlledPawn` (`/Game/01_Scripts/BP_Utils.F_GetPawn`))
  (`/Engine/EditorBlueprintResources/StandardMacros.IsValid` _returnvalue
    (:`Is Valid`
      (`EnhancedInputSubsystemInterface.AddMappingContext` _returnvalue "/Game/01_Scripts/Inputs/IMC_Player.IMC_Player" 0 (struct))
      (`/Game/01_Scripts/BP_GameInstance.E_InitMain` (`/Game/01_Scripts/BP_Utils.F_GetGameInstance`)))))

(event `EnhancedInput|/Game/01_Scripts/Inputs/IA_Movement`
  (params (ActionValue :type "Float (double-precision)") (ElapsedSeconds :type "Float (double-precision)") (TriggeredSeconds :type "Float (double-precision)") (InputAction :type "InputAction Object Reference" :default "/Game/01_Scripts/Inputs/IA_Movement.IA_Movement"))
  (:`Triggered`
    (`/Game/01_Scripts/BP_Pawn.E_Move` (`self.ControlledPawn`) ActionValue)))

(event `EnhancedInput|/Game/01_Scripts/Inputs/IA_Spawn`
  (params (ActionValue :type Boolean) (ElapsedSeconds :type "Float (double-precision)") (TriggeredSeconds :type "Float (double-precision)") (InputAction :type "InputAction Object Reference" :default "/Game/01_Scripts/Inputs/IA_Spawn.IA_Spawn"))
  (:`Triggered`
    (`/Game/01_Scripts/BP_Pawn.E_Spawn` (`self.ControlledPawn`))))

(fn `UserConstructionScript`)