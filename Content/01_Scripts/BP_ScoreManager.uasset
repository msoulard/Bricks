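; BP_ScoreManager keeps the game's score and pushes it to the main UI.
; The E_SetScore event adds a fixed increment through FAddScore, then sends the new total to UIMain, which it reaches through the game instance.
; FResetScore zeroes the score and updates the same UI, while FAddScore alone changes the value without refreshing it.
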(event `E_SetScore`
  (`self.F_AddScore`)
  (`/Game/04_Widgets/UI_Main.F_SetScore` (`/Game/01_Scripts/BP_GameInstance.UIMain` (`/Game/01_Scripts/BP_Utils.F_GetGameInstance`)) (`self.Score`)))

(fn `F_AddScore`
  (set `self.Score` (+ (`self.Score`) 10)))

(fn `F_ResetScore`
  (set `self.Score` 0)
  (`/Game/04_Widgets/UI_Main.F_SetScore` (`/Game/01_Scripts/BP_GameInstance.UIMain` (`/Game/01_Scripts/BP_Utils.F_GetGameInstance`)) (`self.Score`)))

(fn `UserConstructionScript`)